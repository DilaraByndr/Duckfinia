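; Kaz is a duck actor that collects food and loses lives on rotten food, playing a birth flipbook for two seconds before idling.
; Its sphere overlap destroys YEMEK (food) and adds zero to Skor2, so the score never changes.
; ÇÜRÜKYEMEK (rotten food) decrements Can2 and is destroyed, or shows the GameOver widget when one life remains.
; An unconnected node would open GameOverMap but never runs.
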(event OnComponentBeginOverlap(Sphere)
  (params (OverlappedComponent :type Primitive%20Component%20Object%20Reference) (OtherActor :type Actor%20Object%20Reference) (OtherComp :type Primitive%20Component%20Object%20Reference) (OtherBodyIndex :type Integer) (bFromSweep :type Boolean) (SweepResult :type Hit%20Result%20Structure%20%28by%20ref%29))
  (bind _returnvalue (Utilities|GetClass OtherActor))
  (if (== _returnvalue "/Game/Blueprints/YEMEK.YEMEK_C")
    (Variables|Default|Setskor2 (+ 0.0 (Variables|Default|Getskor2)))
    (Development|PrintString (Utilities|String|ToString(Float) 0.0))
    (Actor|DestroyActor OtherActor)
    (elif (== _returnvalue "/Game/Blueprints/ÇÜRÜKYEMEK.ÇÜRÜKYEMEK_C")
      (if (== (Variables|Default|Getcan2) 1)
        (bind _returnvalue_2 (UserInterface|CreateWidget "/Game/UI/GameOver.GameOver_C"))
        (UserInterface|Viewport|AddtoViewport _returnvalue_2 0)
        (else
          (bind _result (Math|Integer|DecrementInt (Variables|Default|Getcan2))
            (:%20%20
              (Development|PrintString "can")
              (Development|PrintString (Utilities|String|ToString(Integer) _result))
              (Actor|DestroyActor OtherActor))))))))

(event EventBeginPlay
  (Sprite|SetFlipbook (Variables|Default|GetWhiteDuck_Birth) "/Game/DuckDuck/WhiteDuck_Birth.WhiteDuck_Birth")
  (Utilities|FlowControl|Delay 2.0)
  (Sprite|SetFlipbook (Variables|Default|GetWhiteDuck_Birth) "/Game/DuckDuck/WhiteDuck_Idle.WhiteDuck_Idle"))

(fn ConstructionScript)